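; Player controller blueprint that pans the Cam pawn along its local forward and right axes from movement axis input.
; On BeginPlay it caches the player pawn as a Cam reference; input is ignored while DisableCamNav is set.
; MovementX and MovementY build the offset transforms, scaling input by FastMoveMultiplier and a clamped speed derived from spring arm length, so movement speeds up as the arm lengthens.
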(event EventBeginPlay
  (Utilities|FlowControl|Sequence
    (:then_0
      (Utilities|ReferenceCasts))))

(event Input|AxisEvents|InputAxisMoveForward
  (params (AxisValue :type Float%20%28single-precision%29))
  (if (not (Variables|Default|GetDisableCamNav))
    (Transformation|SetActorTransform (Variables|References|GetCameraPawnReference) (Utilities|MovementX (CallFunction|MovementSpeedCalculation) (Variables|Default|GetFastMoveMultiplier) AxisValue (Variables|References|GetCameraPawnReference)))))

(event Input|AxisEvents|InputAxisMoveRight
  (params (AxisValue :type Float%20%28single-precision%29))
  (if (not (Variables|Default|GetDisableCamNav))
    (Transformation|SetActorTransform (Variables|References|GetCameraPawnReference) (Utilities|MovementY (CallFunction|MovementSpeedCalculation) (Variables|Default|GetFastMoveMultiplier) AxisValue (Variables|References|GetCameraPawnReference)))))

(fn ConstructionScript)

(fn MovementSpeedCalculation
  (return (Math|Float|Clamp(Float) (/ (Variables|/Script/Engine.SpringArmComponent|GetTargetArmLength (Variables|/Game/Blueprints/Cam.Cam_C|GetSpringArm (Variables|References|GetCameraPawnReference))) 1e+02) 5.0 2e+01)))