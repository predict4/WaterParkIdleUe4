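; IdleGameMode is a game mode Blueprint that runs passive money accumulation for an idle game.
; Tick adds Mps to Money, using the MoneyIncrementing flag and a short Delay to throttle how often the addition happens.
; Each tick also calls ValueToShowUI, which derives a display value and suffix, flooring amounts of a thousand or more to whole thousands with "k".
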(event EventBeginPlay)

(event EventTick
  (params (DeltaSeconds :type Float%20%28single-precision%29))
  ;[1 1 1] Increment Money by 100
  (CallFunction|ValuetoShowUI)
  (if (not (Variables|Default|GetMoneyIncrementing?))
    (Variables|Default|SetMoney (+ (Variables|Default|GetMoney) (Variables|Default|GetMps)))
    (Variables|Default|SetMoneyIncrementing? true)
    (Utilities|FlowControl|Delay 0.1)
    (Variables|Default|SetMoneyIncrementing? false)))

(fn ConstructionScript)

(fn ValuetoShowUI
  (Variables|Default|SetThousands (/ (Variables|Default|GetMoney) 1e+03))
  (if (>= (Variables|Default|GetMoney) 1e+03)
    (Variables|Default|SetValuetoShow (Math|Conversions|ToFloat(Integer) (Math|Float|Floor (Variables|Default|GetThousands))))
    (Variables|Default|SetExponent "k")
    (else
      (Variables|Default|SetValuetoShow (Variables|Default|GetMoney))
      (Variables|Default|SetExponent ""))))